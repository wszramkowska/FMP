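; Behavior tree service for the monster AI that keeps a blackboard flag saying whether the player target is within attack range.
; Each tick it reads the target from the blackboard and checks horizontal distance against AttackRange, plus a fixed height tolerance.
; A visibility line trace must also hit PlayerRef, a variable not assigned in this graph.
; The flag clears when any check fails or the target is invalid.
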(event `self.ReceiveTickAI`
  (params (OwnerController :type "AIController Object Reference") (ControlledPawn :type "Pawn Object Reference") (DeltaSeconds :type "Float (single-precision)"))
  (bind _returnvalue (`Actor.K2_GetActorLocation` ControlledPawn))
  (bind _isinattackrangekey (`self.IsInAttackRangeKey`))
  (bind _asbp_monster_aicontroller (cast `/Game/Dynamic/AI/Monster/Blueprints/BP_MonsterAIController` (`Pawn.GetController` ControlledPawn)))
  (bind _returnvalue_2 (`AIBlueprintHelperLibrary.GetBlackboard` _asbp_monster_aicontroller))
  (bind _returnvalue_3 (`BlackboardComponent.GetValueAsObject` _returnvalue_2 (`self.PlayerTargetKey`)))
  (`/Engine/EditorBlueprintResources/StandardMacros.IsValid` _returnvalue_3
    (:`Is Valid`
      (bind _asbp_third_person_character (cast `/Game/Dynamic/ThirdPerson/Blueprints/BP_ThirdPersonCharacter` _returnvalue_3))
      (bind _returnvalue_4 (`Actor.K2_GetActorLocation` _asbp_third_person_character))
      (bind _outhit (`KismetSystemLibrary.LineTraceSingle` _returnvalue _returnvalue_4 "TraceTypeQuery1"))
      (if (and (< (`KismetMathLibrary.Vector_Distance` (`KismetMathLibrary.MakeVector` (.x _returnvalue) (.y _returnvalue)) (`KismetMathLibrary.MakeVector` (.x _returnvalue_4) (.y _returnvalue_4))) (`self.AttackRange`)) (< (`KismetMathLibrary.Abs` (- (.z _returnvalue_4) (.z _returnvalue))) 150.0) (== (`.HitActor` (`GameplayStatics.BreakHitResult` _outhit)) (`self.PlayerRef`)))
        (`BlackboardComponent.SetValueAsBool` _returnvalue_2 _isinattackrangekey true)
        (else
          (`BlackboardComponent.SetValueAsBool` _returnvalue_2 _isinattackrangekey false))))
    (:`Is Not Valid`
      (`BlackboardComponent.SetValueAsBool` _returnvalue_2 (`self.IsInAttackRangeKey`) false))))