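; Behavior tree service that gradually cools down a monster's aggression level.
; Each AI tick, it casts the controlled pawn's controller to BP_MonsterAIController and reads the aggression blackboard key.
; While that value is above zero, it lowers it by a fixed step per tick, clamped to the valid range, so the decay rate follows the service's tick interval.
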(event `self.ReceiveTickAI`
  (params (OwnerController :type "AIController Object Reference") (ControlledPawn :type "Pawn Object Reference") (DeltaSeconds :type "Float (single-precision)"))
  (bind _asbp_monster_aicontroller (cast `/Game/Dynamic/AI/Monster/Blueprints/BP_MonsterAIController` (`Pawn.GetController` ControlledPawn)))
  (bind _returnvalue (`AIBlueprintHelperLibrary.GetBlackboard` _asbp_monster_aicontroller))
  (bind _returnvalue_2 (`BlackboardComponent.GetValueAsFloat` _returnvalue (`self.AggressionLevelKey`)))
  (if (> _returnvalue_2 0.0)
    (`BlackboardComponent.SetValueAsFloat` _returnvalue (`self.AggressionLevelKey`) (`KismetMathLibrary.FClamp` (- _returnvalue_2 0.5) 0.0 100.0))))