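; Behavior tree task that picks a random patrol destination for a monster AI.
; It gathers all BP_PatrolPoint actors in the level and writes a random one's location to the patrol point blackboard key via BP_MonsterAIController, then finishes successfully.
; With no patrol points it only prints a message and never finishes; a failed controller cast also leaves the task unfinished.
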(event `self.ReceiveExecuteAI`
  (params (OwnerController :type "AIController Object Reference") (ControlledPawn :type "Pawn Object Reference"))
  (bind _outactors (`GameplayStatics.GetAllActorsOfClass` "/Game/Dynamic/AI/Monster/Blueprints/BP_PatrolPoint.BP_PatrolPoint_C"))
  (bind _returnvalue (`KismetArrayLibrary.Array_Length` _outactors))
  (if (> _returnvalue 0)
    (bind _asbp_monster_aicontroller (cast `/Game/Dynamic/AI/Monster/Blueprints/BP_MonsterAIController` (`Pawn.GetController` ControlledPawn)))
    (`BlackboardComponent.SetValueAsVector` (`AIBlueprintHelperLibrary.GetBlackboard` _asbp_monster_aicontroller) (`self.PatrolPointKey`) (`Actor.K2_GetActorLocation` (`|GetArrayItem` _outactors (`KismetMathLibrary.RandomIntegerInRange` 0 (- _returnvalue 1)))))
    (`self.FinishExecute` true)
    (else
      (`KismetSystemLibrary.PrintString` "No Patrol Points"))))