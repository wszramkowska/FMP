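; Behavior tree task for the monster AI that stands in for an area search, ending an investigation that finds nothing.
; It waits briefly, then lowers the clamped aggression value and clears the investigating flag on the monster controller's blackboard.
; It prints a debug message and finishes successfully, with no movement or detection logic of its own.
; A failed controller cast leaves the task without a finish call.
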(event `self.ReceiveExecuteAI`
  (params (OwnerController :type "AIController Object Reference") (ControlledPawn :type "Pawn Object Reference"))
  (`KismetSystemLibrary.Delay` 2.0)
  (bind _asbp_monster_aicontroller (cast `/Game/Dynamic/AI/Monster/Blueprints/BP_MonsterAIController` (`Pawn.GetController` ControlledPawn)))
  (bind _returnvalue (`AIBlueprintHelperLibrary.GetBlackboard` _asbp_monster_aicontroller))
  (`BlackboardComponent.SetValueAsFloat` _returnvalue (`self.AggressionLevelKey`) (`KismetMathLibrary.FClamp` (- (`BlackboardComponent.GetValueAsFloat` _returnvalue (`self.AggressionLevelKey`)) 5.0) 0.0 100.0))
  (`BlackboardComponent.SetValueAsBool` _returnvalue (`self.IsInvestigatingKey`) false)
  (`KismetSystemLibrary.PrintString` "Search done: nothing found")
  (`self.FinishExecute` true))