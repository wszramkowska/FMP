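; Behavior tree task that moves the monster to the player stored in the blackboard, branching on whether the in-light flag is set.
; Both branches record the player's position as last known; the dark branch also clears the hunting flag, and its move has no Pawn input.
; The move result finishes the task; a failed player cast clears hunting and fails, while an invalid target never finishes it.
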(event `self.ReceiveExecuteAI`
  (params (OwnerController :type "AIController Object Reference") (ControlledPawn :type "Pawn Object Reference"))
  (bind _returnvalue (`AIBlueprintHelperLibrary.GetBlackboard` ControlledPawn))
  (bind _asbp_monster_aicontroller (cast `/Game/Dynamic/AI/Monster/Blueprints/BP_MonsterAIController` (`Pawn.GetController` ControlledPawn)))
  (bind _returnvalue_2 (`AIBlueprintHelperLibrary.GetBlackboard` _asbp_monster_aicontroller))
  (bind _returnvalue_3 (`BlackboardComponent.GetValueAsObject` _returnvalue_2 (`self.PlayerTargetKey`)))
  (`/Engine/EditorBlueprintResources/StandardMacros.IsValid` _returnvalue_3
    (:`Is Valid`
      (bind _asbp_third_person_character (cast `/Game/Dynamic/ThirdPerson/Blueprints/BP_ThirdPersonCharacter` _returnvalue_3)
        (:`then`
          (if (`BlackboardComponent.GetValueAsBool` _returnvalue_2 (`self.IsInLightKey`))
            (`KismetSystemLibrary.PrintString` "IN LIGHT")
            (bind _returnvalue_4 (`Actor.K2_GetActorLocation` _asbp_third_person_character))
            (`BlackboardComponent.SetValueAsVector` _returnvalue_2 (`self.LastKnownPlayerLocationKey`) _returnvalue_4)
            (`|AIMoveTo` ControlledPawn _returnvalue_4 null 100.0
              (:`OnSuccess`
                (`self.FinishExecute` true))
              (:`OnFail`
                (`self.FinishExecute` false)))
            (else
              (`KismetSystemLibrary.PrintString` "IN DARK")
              (`BlackboardComponent.SetValueAsVector` _returnvalue (`self.LastKnownPlayerLocationKey`) _returnvalue_4)
              (`BlackboardComponent.SetValueAsBool` _returnvalue (`self.IsHuntingKey`) false)
              (`|AIMoveTo` null _returnvalue_4 null
                (:`OnSuccess`
                  (`self.FinishExecute` true))
                (:`OnFail`
                  (`self.FinishExecute` false))))))
        (:`CastFailed`
          (`BlackboardComponent.SetValueAsBool` _returnvalue_2 (`self.IsHuntingKey`) false)
          (`self.FinishExecute` false))))))