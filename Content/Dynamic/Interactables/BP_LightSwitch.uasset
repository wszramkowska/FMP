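; BP_LightSwitch is an interactable light switch that toggles an array of linked lights on and off.
; On Interaction it plays a click sound, reports a "LightSwitch" noise event that AI hearing can pick up, tilts the switch mesh and flips each light's visibility.
; The construction script matches the switch angle and light visibility to the LightOn flag, so the initial state shows in the editor.
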(event `/Game/Dynamic/Interfaces/BPI_Interaction.Interaction`
  (bind _lightswitch (`self.LightSwitch`))
  (bind _relativelocation (`SceneComponent.RelativeLocation` _lightswitch))
  ; Turning Lights On or Off
  (`GameplayStatics.PlaySound2D` "/Game/Static/Audio/485063__joncon_library__switch_02.485063__joncon_library__switch_02" 1.0 1.0 0.0 null null)
  (`AISense_Hearing.ReportNoiseEvent` (`self.K2_GetActorLocation`) 10.0 self 3000.0 "LightSwitch")
  (if (`self.LightOn`)
    (`KismetSystemLibrary.MoveComponentTo` _lightswitch _relativelocation (`KismetMathLibrary.MakeRotator` 30.0) false false 0.1)
    (for _array_element (`self.Lights`)
      (`SceneComponent.SetVisibility` (`Light.LightComponent` _array_element) false false)
      (set `self.LightOn` false))
    (else
      (`KismetSystemLibrary.MoveComponentTo` _lightswitch _relativelocation (`KismetMathLibrary.MakeRotator` -30.0) false false 0.1)
      (for _array_element_2 (`self.Lights`)
        (`SceneComponent.SetVisibility` (`Light.LightComponent` _array_element_2) true false)
        (set `self.LightOn` true)))))

(fn `UserConstructionScript`
  (if (`self.LightOn`)
    (`SceneComponent.K2_SetRelativeRotation` (`self.LightSwitch`) (`KismetMathLibrary.MakeRotator` -30.0) false false)
    (for _array_element (`self.Lights`)
      (`SceneComponent.SetVisibility` (`Light.LightComponent` _array_element) true false))
    (else
      (`SceneComponent.K2_SetRelativeRotation` (`self.LightSwitch`) (`KismetMathLibrary.MakeRotator` 30.0) false false)
      (for _array_element_2 (`self.Lights`)
        (`SceneComponent.SetVisibility` (`Light.LightComponent` _array_element_2) false false)))))