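; BP_NightlightSocket is the interactable socket where the player assembles the nightlight to end the horror game.
; Interaction checks GI_Horror for four collected pieces, showing a timed progress prompt if any are missing.
; Otherwise it locks player input, plays the skeletal-mesh assembly animations and enables doorway blocker collision.
; Delays and timelines chain the GameInstance notifications into a warm light bloom and a final view-target blend.
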(event `self.ReceiveEndPlay`
  (params (EndPlayReason :type "EEndPlayReason Enum" :default "Destroyed"))
  (bind _interactpromptwidget (`self.InteractPromptWidget`))
  (`/Engine/EditorBlueprintResources/StandardMacros.IsValid` _interactpromptwidget
    (:`Is Valid`
      (`Widget.RemoveFromParent` _interactpromptwidget))))

(event `self.ReceiveBeginPlay`
  (bind _asgi_horror (cast `/Game/Dynamic/ThirdPerson/Blueprints/GI_Horror` (`GameplayStatics.GetGameInstance`)))
  (set `self.GIHorrorRef` _asgi_horror))

(event `HidePrompt`
  (`KismetSystemLibrary.PrintString` "4 SECONDS DONE" true true (struct :`R` 0.039822 :`B` 1.0 :`A` 1.0))
  (`Widget.RemoveFromParent` (`self.InteractPromptWidget`)))

(event `/Game/Dynamic/Interfaces/BPI_Interaction.Interaction`
  (bind _returnvalue (`GameplayStatics.GetPlayerController` 0))
  (bind _interactpromptwidget (`self.InteractPromptWidget`))
  (if (`self.AssemblyStarted?`)
    _
    (elif (== (`/Game/Dynamic/ThirdPerson/Blueprints/GI_Horror.PiecesCollected` (`self.GIHorrorRef`)) 4)
      (set `self.AssemblyStarted?` true)
      (`Controller.SetIgnoreMoveInput` _returnvalue true)
      (`Controller.SetIgnoreLookInput` _returnvalue true)
      (`/Game/Dynamic/ThirdPerson/Blueprints/GI_Horror.OnAssemblyBegin` (`self.GIHorrorRef`))
      (`self.BeginAssemblySequence`)
      (else
        (`KismetSystemLibrary.PrintString` "You need all the pieces")
        (`/Engine/EditorBlueprintResources/StandardMacros.IsValid` _interactpromptwidget
          (:`Is Valid`
            _)
          (:`Is Not Valid`
            _))
        (if (not (`Widget.IsInViewport` _interactpromptwidget))
          (bind _returnvalue_2 (`|CreateWidget` "/Game/Dynamic/UI/WB_InteractPrompt.WB_InteractPrompt_C"))
          (bind _output_get (set `self.InteractPromptWidget` _returnvalue_2))
          (`UserWidget.AddToViewport` _output_get 0))
        (`/Game/Dynamic/UI/WB_InteractPrompt.UpdatePiecesCollected` _interactpromptwidget)
        (`KismetSystemLibrary.K2_ClearAndInvalidateTimerHandle` (`self.TimerHandle`))
        (bind _returnvalue_3 (`KismetSystemLibrary.K2_SetTimer` null "HidePrompt" 4.0))
        (set `self.TimerHandle` _returnvalue_3)))))

(event `BeginAssemblySequence`
  (`self.PlayEndingAnim`)
  (`/Game/Dynamic/ThirdPerson/Blueprints/GI_Horror.OnBulbInserted` (`self.GIHorrorRef`))
  (`KismetSystemLibrary.PrintString` "BULB INSERTED")
  (`PrimitiveComponent.SetCollisionEnabled` (`Brush.BrushComponent` (`self.DoorwayBlocker`)) "QueryAndPhysics")
  (`KismetSystemLibrary.Delay` 0.5)
  (`Timeline|Step_4`
    (:`Finished`
      (`KismetSystemLibrary.Delay` 5.0)
      (`/Game/Dynamic/ThirdPerson/Blueprints/GI_Horror.OnNightlightComplete` (`self.GIHorrorRef`))
      (`KismetSystemLibrary.PrintString` "NIGHTLIGHT COMPELTE")
      (`self.BeginWinState`))))

(event `BeginWinState`
  (`LightComponent.SetLightColor` (`self.SocketGlowLight`) (make `LinearColor` 1.0 0.6 0.2 1.0) true)
  (bind (_direction _alpha) (`Timeline|LightBloom`)
    (:`Update`
      (`LightComponent.SetIntensity` (`self.SocketGlowLight`) (* _alpha 8000.0)))
    (:`Finished`
      (`KismetSystemLibrary.Delay` 3.0)
      (`PlayerController.SetViewTargetWithBlend` (`GameplayStatics.GetPlayerController` 0) null 0.0 "VTBlend_Linear" 0.0 false)
      (`KismetSystemLibrary.Delay` 1.0))))

(fn `PlayEndingAnim`
  (bind _skeletalmeshcomponent (`SkeletalMeshActor.SkeletalMeshComponent` (`self.SKM_Bulb`)))
  (bind _skeletalmeshcomponent_2 (`SkeletalMeshActor.SkeletalMeshComponent` (`self.SKM_Bottom`)))
  (bind _skeletalmeshcomponent_3 (`SkeletalMeshActor.SkeletalMeshComponent` (`self.SKM_Top`)))
  (bind _skeletalmeshcomponent_4 (`SkeletalMeshActor.SkeletalMeshComponent` (`self.SKM_Switch`)))
  (bind _skeletalmeshcomponent_5 (`SkeletalMeshActor.SkeletalMeshComponent` (`self.SKM_SwitchBase`)))
  (`SceneComponent.SetVisibility` _skeletalmeshcomponent true false)
  (`SceneComponent.SetVisibility` _skeletalmeshcomponent_2 true false)
  (`SceneComponent.SetVisibility` _skeletalmeshcomponent_3 true false)
  (`SceneComponent.SetVisibility` _skeletalmeshcomponent_4 true false)
  (`SceneComponent.SetVisibility` _skeletalmeshcomponent_5 true false)
  (`SkeletalMeshComponent.PlayAnimation` _skeletalmeshcomponent "/Game/Dynamic/Anims/Nightlight/SK_Bulb_Anim.SK_Bulb_Anim" false)
  (`SkeletalMeshComponent.PlayAnimation` _skeletalmeshcomponent_2 "/Game/Dynamic/Anims/Nightlight/SK_Base_Anim.SK_Base_Anim" false)
  (`SkeletalMeshComponent.PlayAnimation` _skeletalmeshcomponent_3 "/Game/Dynamic/Anims/Nightlight/SK_Fuse_Anim.SK_Fuse_Anim" false)
  (`SkeletalMeshComponent.PlayAnimation` _skeletalmeshcomponent_4 "/Game/Dynamic/Anims/Nightlight/SK_Switch_Anim.SK_Switch_Anim" false)
  (`SkeletalMeshComponent.PlayAnimation` _skeletalmeshcomponent_5 "/Game/Dynamic/Anims/Nightlight/SK_Switchbase_Anim.SK_Switchbase_Anim" false))

(fn `UserConstructionScript`)