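; BP_Nightlight is an interactable nightlight pickup that counts as a collectible piece in a horror game.
; Interaction calls HandlePickup, which acts once, and only while IsUnlocked is true.
; It sets IsPickedUp, plays a sound at world origin, hides the mesh without destroying the actor, and registers PieceID with the GI_Horror game instance cached at BeginPlay.
; Debug strings print the pickup and the collected piece count.
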(event `self.ReceiveBeginPlay`
  (bind _asgi_horror (cast `/Game/Dynamic/ThirdPerson/Blueprints/GI_Horror` (`GameplayStatics.GetGameInstance`)))
  (set `self.GIHorrorRef` _asgi_horror))

(event `/Game/Dynamic/Interfaces/BPI_Interaction.Interaction`
  (`self.HandlePickup`))

(fn `HandlePickup`
  (if (`self.IsUnlocked?`)
    (if (not (`self.IsPickedUp?`))
      (set `self.IsPickedUp?` true)
      (`GameplayStatics.PlaySoundAtLocation` null (0.0 0.0 0.0) (struct) 1.0 1.0 0.0 null null null null)
      (`SceneComponent.SetHiddenInGame` (`self.StaticMesh`) true false)
      (`/Game/Dynamic/ThirdPerson/Blueprints/GI_Horror.RegisterPiece` (`self.GIHorrorRef`) (`self.PieceID`))
      (`KismetSystemLibrary.PrintString` "PICKED UP")
      (`KismetSystemLibrary.PrintString` (`KismetStringLibrary.Concat_StrStr` "Pieces collected: " (`KismetStringLibrary.Conv_IntToString` (`/Game/Dynamic/ThirdPerson/Blueprints/GI_Horror.PiecesCollected` (`self.GIHorrorRef`))))))))

(fn `UserConstructionScript`)