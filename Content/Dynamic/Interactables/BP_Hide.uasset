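; BP_Hide is an interactable hiding spot that pulls the player character into a set position.
; On Interaction, it disables the player's collision and movement, then starts a looping timer ticking at the current frame's delta time.
; Each timer tick moves the player at constant speed toward the PlayerPosition component, clearing the timer on arrival.
; The file contains no logic for leaving the spot or restoring collision and movement.
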(event `self.ReceiveBeginPlay`
  (bind _asbp_third_person_character (cast `/Game/Dynamic/ThirdPerson/Blueprints/BP_ThirdPersonCharacter` (`GameplayStatics.GetPlayerCharacter` 0)))
  (set `self.PlayerRef` _asbp_third_person_character))

(event `/Game/Dynamic/Interfaces/BPI_Interaction.Interaction`
  (bind _playerref (`self.PlayerRef`))
  ; Hiding Logic
  (`self.SetActorEnableCollision` _playerref false)
  (`CharacterMovementComponent.DisableMovement` (`Character.CharacterMovement` _playerref))
  (bind _returnvalue (`KismetSystemLibrary.K2_SetTimerDelegate` (delegate `MoveCharacter`) (`GameplayStatics.GetWorldDeltaSeconds`) true)))

(event `MoveCharacter`
  (bind _playerref (`self.PlayerRef`))
  ; Hiding Logic
  (`self.K2_SetActorTransform` _playerref (`KismetMathLibrary.MakeTransform` (`KismetMathLibrary.VInterpTo_Constant` (`self.K2_GetActorLocation` _playerref) (`SceneComponent.K2_GetComponentLocation` (`self.PlayerPosition`)) (`GameplayStatics.GetWorldDeltaSeconds`) 1000.0)) false false)
  (if (== (`SceneComponent.K2_GetComponentLocation` (`self.PlayerPosition`)) (`self.K2_GetActorLocation` (`self.PlayerRef`)))
    (`KismetSystemLibrary.K2_ClearAndInvalidateTimerHandle` (stale `/Game/Dynamic/Interfaces/BPI_Interaction.Interaction` _returnvalue))))

(fn `UserConstructionScript`)