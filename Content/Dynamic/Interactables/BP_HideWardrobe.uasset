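; Interactable hiding wardrobe, a child Blueprint that adds swinging double doors to its parent's interaction logic.
; Interaction locks out repeat use, plays the player's open-wardrobe animation and a sound, then opens both doors with a timeline before calling the parent Interaction.
; The HidingED dispatcher, bound on BeginPlay, triggers a second timeline that closes the doors and re-enables interaction when finished.
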(event `self.ReceiveBeginPlay`
  (bind _asbp_third_person_character (cast `/Game/Dynamic/ThirdPerson/Blueprints/BP_ThirdPersonCharacter` (`GameplayStatics.GetPlayerCharacter` 0)))
  (set `self.CharacterRef` _asbp_third_person_character)
  (`parent.ReceiveBeginPlay`)
  (add `self.HidingED` (delegate `HidingED_Event`)))

(event `HidingED_Event`
  (`self.CloseDoor`))

(event `/Game/Dynamic/Interfaces/BPI_Interaction.Interaction`
  (if (`self.CanInteract?`)
    (set `self.CanInteract?` false)
    (`/Game/Dynamic/ThirdPerson/Blueprints/BP_ThirdPersonCharacter.PlayOpenWardrobeAnim` (`self.CharacterRef`))
    (`GameplayStatics.PlaySound2D` "/Game/Static/Audio/short-fire-whoosh_1-317280.short-fire-whoosh_1-317280" 1.0 1.0 0.0 null null)
    (bind (_direction _alpha) (`Timeline|OpenDoor` :!via `PlayFromStart`)
      (:`Update`
        (`SceneComponent.K2_SetRelativeRotation` (`self.DoorRMesh`) (`KismetMathLibrary.MakeRotator` 0.0 0.0 (`KismetMathLibrary.Lerp` 0.0 -100.0 _alpha)) false false)
        (`SceneComponent.K2_SetRelativeRotation` (`self.DoorLMesh`) (`KismetMathLibrary.MakeRotator` 0.0 0.0 (`KismetMathLibrary.Lerp` 0.0 100.0 _alpha)) false false))
      (:`Finished`
        (`parent.Interaction`)))))

(event `CloseDoor`
  (bind (_direction _alpha) (`Timeline|CloseWardrobeDoor` :!via `PlayFromStart`)
    (:`Update`
      (`SceneComponent.K2_SetRelativeRotation` (`self.DoorRMesh`) (`KismetMathLibrary.MakeRotator` 0.0 0.0 (`KismetMathLibrary.Lerp` -100.0 0.0 _alpha)) false false)
      (`SceneComponent.K2_SetRelativeRotation` (`self.DoorLMesh`) (`KismetMathLibrary.MakeRotator` 0.0 0.0 (`KismetMathLibrary.Lerp` 100.0 0.0 _alpha)) false false))
    (:`Finished`
      (set `self.CanInteract?` true))))

(fn `UserConstructionScript`
  (`parent.UserConstructionScript`))